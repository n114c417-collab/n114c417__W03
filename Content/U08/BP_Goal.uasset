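; BP_Goal is a level goal that shows the win screen when the My_dog02 actor reaches it.
; The first overlap of its Trigger by that actor passes a DoOnce, waits briefly, prints a congratulation message, adds WBP_WinScreen to the viewport and shows the mouse cursor.
; Nodes for reloading the current level are present but unconnected, so they never run.
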(event `self.Trigger.OnComponentBeginOverlap`
  (params (OverlappedComponent :type "PrimitiveComponent Object Reference") (OtherActor :type "Actor Object Reference") (OtherComp :type "PrimitiveComponent Object Reference") (OtherBodyIndex :type Integer) (bFromSweep :type Boolean) (SweepResult :type "HitResult Structure (by ref)"))
  (cast `/Game/U05/My_dog02` OtherActor)
  (`/Engine/EditorBlueprintResources/StandardMacros.DoOnce` false
    (:`Completed`
      (`KismetSystemLibrary.Delay` 0.1)
      (`KismetSystemLibrary.PrintString` "恭喜通關")
      (bind _returnvalue (`|CreateWidget` "/Game/U08/WBP_WinScreen.WBP_WinScreen_C"))
      (`UserWidget.AddToViewport` _returnvalue 0)
      (set `PlayerController.bShowMouseCursor` true (`GameplayStatics.GetPlayerController` 0)))))

(fn `UserConstructionScript`)