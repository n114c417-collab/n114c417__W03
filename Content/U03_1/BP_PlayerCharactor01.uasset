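; Player character Blueprint for side-scrolling movement along the world X axis with jumping, driven by Enhanced Input.
; BeginPlay adds the IMC_Player01 mapping context, and the jump action starts and stops the built-in Jump.
; The move action, gated by CanMove, feeds movement input and sets IsFacingRight, which flips PlayerSprite by rotating it 180 degrees.
; Print strings trace walking, jumping and locked movement for debugging.
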(event `self.ReceiveBeginPlay`
  (`EnhancedInputSubsystemInterface.AddMappingContext` (pcsubsystem `EnhancedInputLocalPlayerSubsystem` (`GameplayStatics.GetPlayerController` 0)) "/Game/U03_1/Input/IMC_Player01.IMC_Player01" 0 (struct)))

(event `EnhancedInput|/Game/U03_1/Input/IA_Move01`
  (params (ActionValue :type "Vector2D Structure") (ElapsedSeconds :type "Float (double-precision)") (TriggeredSeconds :type "Float (double-precision)") (InputAction :type "InputAction Object Reference" :default "/Game/U03_1/Input/IA_Move01.IA_Move01"))
  (bind _x (`KismetMathLibrary.BreakVector2D` ActionValue))
  (bind _playersprite (`self.PlayerSprite`))
  (:`Triggered`
    (if (`self.CanMove`)
      (if (> _x 0.0)
        (set `self.isFacingRight` true)
        (else
          (set `self.isFacingRight` false)))
      (`self.AddMovementInput` (1.0 0.0 0.0) _x)
      (if (`self.isFacingRight`)
        (`SceneComponent.K2_SetRelativeRotation` :`self` _playersprite)
        (`KismetSystemLibrary.PrintString` "Walk Right" true true (struct :`G` 0.66 :`B` 1.0 :`A` 1.0) 2.0 "1")
        (else
          (`SceneComponent.K2_SetRelativeRotation` _playersprite (struct :`Yaw` 180.0) false false)
          (`KismetSystemLibrary.PrintString` "Walk Left" true true (struct :`G` 0.66 :`B` 1.0 :`A` 1.0) 2.0 "1")))
      (else
        (`KismetSystemLibrary.PrintString` "movelocked")))))

(event `EnhancedInput|/Game/U03_1/Input/IA_Jump01`
  (params (ActionValue :type Boolean) (ElapsedSeconds :type "Float (double-precision)") (TriggeredSeconds :type "Float (double-precision)") (InputAction :type "InputAction Object Reference" :default "/Game/U03_1/Input/IA_Jump01.IA_Jump01"))
  (:`Started`
    (`self.Jump`)
    (`KismetSystemLibrary.PrintString` "Jump" true true (struct :`G` 0.66 :`B` 1.0 :`A` 1.0) 2.0 "1" :!label _label))
  (:`Completed`
    (`self.StopJumping`)
    (goto _label)))

(fn `UserConstructionScript`)